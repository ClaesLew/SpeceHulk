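; BP_Lift is a lift that moves between its starting relative position and Endpos when the player enters its trigger.
; After a short delay, a FlipFlop alternately plays and reverses the Move timeline on successive player overlaps.
; The timeline's alpha lerps the Lift component's relative location from zero to Endpos, with Time setting the play rate.
; End overlap only casts to the player and takes no action.
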(event OnComponentBeginOverlap(Trigger)
  (params (OverlappedComponent :type Primitive%20Component%20Object%20Reference) (OtherActor :type Actor%20Object%20Reference) (OtherComp :type Primitive%20Component%20Object%20Reference) (OtherBodyIndex :type Integer) (bFromSweep :type Boolean) (SweepResult :type Hit%20Result%20Structure%20%28by%20ref%29))
  (Utilities|Casting|CastToCore_PlayerCharacter OtherActor)
  (Utilities|FlowControl|Delay 0.2)
  (Utilities|FlowControl|FlipFlop
    (:A
      (bind _alpha (Timeline|Move Play)
        (:Update
          (Transformation|SetRelativeLocation (Variables|Default|Getlift) (Math|Vector|Lerp(Vector) "0, 0, 0" (Variables|Default|GetEndpos) _alpha) false false))))
    (:B
      (Timeline|Move Reverse))))

(event OnComponentEndOverlap(Trigger)
  (params (OverlappedComponent :type Primitive%20Component%20Object%20Reference) (OtherActor :type Actor%20Object%20Reference) (OtherComp :type Primitive%20Component%20Object%20Reference) (OtherBodyIndex :type Integer))
  (Utilities|Casting|CastToCore_PlayerCharacter OtherActor))

(event EventBeginPlay
  (Components|Timeline|SetPlayRate (Variables|Default|GetMove) (Variables|Default|GetTime)))

(fn ConstructionScript)