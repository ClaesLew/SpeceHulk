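; BP_DamageTrigger is a trigger volume that deals periodic damage to the player while they are inside it.
; Overlap begin caches the Core_PlayerCharacter and starts a looping timer at DamageInterval, with no damage on entry itself.
; Each tick of that timer applies DamageDealt to the cached player.
; Overlap end pauses the timer by its stored handle rather than clearing it.
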(event OnComponentBeginOverlap(Trigger)
  (params (OverlappedComponent :type Primitive%20Component%20Object%20Reference) (OtherActor :type Actor%20Object%20Reference) (OtherComp :type Primitive%20Component%20Object%20Reference) (OtherBodyIndex :type Integer) (bFromSweep :type Boolean) (SweepResult :type Hit%20Result%20Structure%20%28by%20ref%29))
  (bind _ascore_player_character (Utilities|Casting|CastToCore_PlayerCharacter OtherActor))
  (bind _returnvalue (Utilities|Time|SetTimerbyEvent (delegate Custom|OnPlayerInsideTrigger) (Variables|Default|GetDamage%20Interval) true))
  (Variables|Default|SetTimerDamgeDealer _returnvalue))

(event OnComponentEndOverlap(Trigger)
  (params (OverlappedComponent :type Primitive%20Component%20Object%20Reference) (OtherActor :type Actor%20Object%20Reference) (OtherComp :type Primitive%20Component%20Object%20Reference) (OtherBodyIndex :type Integer))
  (Utilities|Casting|CastToCore_PlayerCharacter OtherActor)
  (Utilities|Time|PauseTimerbyHandle (Variables|Default|GetTimerDamgeDealer)))

(event Custom|OnPlayerInsideTrigger
  (Game|Damage|ApplyDamage (stale OnComponentBeginOverlap(Trigger) _ascore_player_character) (Variables|Default|GetDamageDealt) 0 0))

(fn ConstructionScript)