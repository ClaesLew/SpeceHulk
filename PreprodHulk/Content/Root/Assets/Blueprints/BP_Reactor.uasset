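; BP_Reactor is a level 4 objective that the player takes by overlapping its trigger.
; A player overlap destroys the reactor piece, then once only prints the reactor number, stops the Machine timeline, increments ReactorTaken on the game instance and calls WinLvl4.
; The Machine timeline's update spins the top and bottom parts opposite to the piece, though no graph event starts it.
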(event OnComponentBeginOverlap(Triggger)
  (params (OverlappedComponent :type Primitive%20Component%20Object%20Reference) (OtherActor :type Actor%20Object%20Reference) (OtherComp :type Primitive%20Component%20Object%20Reference) (OtherBodyIndex :type Integer) (bFromSweep :type Boolean) (SweepResult :type Hit%20Result%20Structure%20%28by%20ref%29))
  (Utilities|Casting|CastToCore_PlayerCharacter OtherActor)
  (Components|DestroyComponent (Variables|Default|Getreactorpeice))
  (Utilities|FlowControl|DoOnce false
    (:Completed
      (Development|PrintString (Variables|Default|GetReactor%20number))
      (Audio|Components|Audio|Stop (Variables|Default|GetMachine))
      (bind _ascore_game_instance (Utilities|Casting|CastToCore_GameInstance (Game|GetGameInstance)))
      (Math|Integer|IncrementInt (Variables|/Game/Root/Core/FrameWork/Core_GameInstance.Core_GameInstance_C|GetReactorTaken _ascore_game_instance)
        (:%20%20
          (Default|WinLvl4 _ascore_game_instance))))))

(fn ConstructionScript)