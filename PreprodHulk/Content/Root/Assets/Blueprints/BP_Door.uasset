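; BP_Door is a sliding double door that opens when something overlaps its Box trigger and closes when the overlap ends, provided its Open flag is set.
; The DoorOpen timeline lerps the left and right panels from a shared start position to their end positions, reversing to close.
; When Usable is set, BeginPlay calls LightStates, which makes the frame's light material green if Open, otherwise the default.
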(event OnComponentBeginOverlap(Box)
  (params (OverlappedComponent :type Primitive%20Component%20Object%20Reference) (OtherActor :type Actor%20Object%20Reference) (OtherComp :type Primitive%20Component%20Object%20Reference) (OtherBodyIndex :type Integer) (bFromSweep :type Boolean) (SweepResult :type Hit%20Result%20Structure%20%28by%20ref%29))
  (bind _startpos (Variables|Default|GetStartPos))
  (if (Variables|Default|GetbOpen)
    (bind _alpha (Timeline|DoorOpen Play)
      (:Update
        (Transformation|SetRelativeLocation (Variables|Default|GetDLeft) (Math|Vector|Lerp(Vector) _startpos (Variables|Default|GetEndPosLeft) _alpha) false false)
        (Transformation|SetRelativeLocation (Variables|Default|GetDRight) (Math|Vector|Lerp(Vector) _startpos (Variables|Default|GetEndPosRight) _alpha) false false)))))

(event OnComponentEndOverlap(Box)
  (params (OverlappedComponent :type Primitive%20Component%20Object%20Reference) (OtherActor :type Actor%20Object%20Reference) (OtherComp :type Primitive%20Component%20Object%20Reference) (OtherBodyIndex :type Integer))
  (bind _startpos (Variables|Default|GetStartPos))
  (if (Variables|Default|GetbOpen)
    (bind _alpha (Timeline|DoorOpen Reverse)
      (:Update
        (Transformation|SetRelativeLocation (Variables|Default|GetDLeft) (Math|Vector|Lerp(Vector) _startpos (Variables|Default|GetEndPosLeft) _alpha) false false)
        (Transformation|SetRelativeLocation (Variables|Default|GetDRight) (Math|Vector|Lerp(Vector) _startpos (Variables|Default|GetEndPosRight) _alpha) false false)))))

(event EventBeginPlay
  (if (Variables|Default|GetbUsable)
    (CallFunction|LightStates)))

(fn ConstructionScript)

(fn LightStates
  (bind _frame (Variables|Default|GetFrame))
  (if (Variables|Default|GetbOpen)
    (Rendering|Material|SetMaterial _frame 1 "/Game/Root/Assets/Materials/M_Color_Master_Inst_Green.M_Color_Master_Inst_Green")
    (else
      (Rendering|Material|SetMaterial _frame 1 "/Game/Root/Assets/Materials/M_Color_Master.M_Color_Master"))))