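; BP_CardMachine is a trigger-driven card machine that opens a referenced tunnel door when the game instance reports the yellow card.
; Entering the trigger shows the card, cube and text render, and with the card also calls OpenDoor on BP_Tunnel and swaps the text.
; Leaving hides those components only if the card is missing.
; The CardMov timeline that would rotate Pivot is never run.
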(event OnComponentBeginOverlap(Trigger)
  (params (OverlappedComponent :type Primitive%20Component%20Object%20Reference) (OtherActor :type Actor%20Object%20Reference) (OtherComp :type Primitive%20Component%20Object%20Reference) (OtherBodyIndex :type Integer) (bFromSweep :type Boolean) (SweepResult :type Hit%20Result%20Structure%20%28by%20ref%29))
  (bind _ascore_game_instance (Utilities|Casting|CastToCore_GameInstance (Game|GetGameInstance)))
  (if (Variables|/Game/Root/Core/FrameWork/Core_GameInstance.Core_GameInstance_C|GetbHasYellowCard _ascore_game_instance)
    (bind _asbp_tunnel (Utilities|Casting|CastToBP_Tunnel (Variables|Default|GetTunnelref)))
    (Default|OpenDoor _asbp_tunnel)
    (Rendering|Components|TextRender|SetText (Variables|Default|GetTextRender) (Variables|Default|GetTextchange))
    (Rendering|SetVisibility (Variables|Default|GetCard) true false)
    (else
      (Rendering|SetVisibility (Variables|Default|GetCard) true false))))

(event OnComponentEndOverlap(Trigger)
  (params (OverlappedComponent :type Primitive%20Component%20Object%20Reference) (OtherActor :type Actor%20Object%20Reference) (OtherComp :type Primitive%20Component%20Object%20Reference) (OtherBodyIndex :type Integer))
  (if (not (Variables|/Game/Root/Core/FrameWork/Core_GameInstance.Core_GameInstance_C|GetbHasYellowCard (stale OnComponentBeginOverlap(Trigger) _ascore_game_instance)))
    (Rendering|SetVisibility (Variables|Default|GetCard) false false)))

(fn ConstructionScript)