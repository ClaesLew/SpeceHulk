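; BP_EggInge is a shootable egg actor that loses one Life each time a FirstPersonProjectile hits its Collision component.
; When Life reaches zero, DEATH stops Timeline_0, which drives a slight vertical stretch of the Eggs component.
; It then plays the Deathanim timeline to squash Eggs wide and flat.
; A five-second delay triggered from that timeline's update leads to destroying the actor.
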(event OnComponentHit(Collision)
  (params (HitComponent :type Primitive%20Component%20Object%20Reference) (OtherActor :type Actor%20Object%20Reference) (OtherComp :type Primitive%20Component%20Object%20Reference) (NormalImpulse :type Vector :default "0, 0, 0") (Hit :type Hit%20Result%20Structure%20%28by%20ref%29))
  (bind _life (Variables|Default|GetLife))
  (Utilities|Casting|CastToFirstPersonProjectile OtherActor)
  (Math|Integer|DecrementInt _life
    (:%20%20
      (if (== _life 0)
        (CallFunction|DEATH)))))

(event Custom|DEATH
  (Utilities|FlowControl|Sequence
    (:then_0
      (bind _alpha (Timeline|Timeline_0 Stop)
        (:Update
          (Transformation|SetRelativeScale3D (Variables|Default|GetEggs) (Math|Vector|Lerp(Vector) "1.000000,1.000000,1.000000" "1.000000,1.000000,1.050000" _alpha)))))
    (:then_1
      (bind _newtrack_0 (Timeline|Deathanim Play)
        (:Update
          (Transformation|SetRelativeScale3D (Variables|Default|GetEggs) (Math|Vector|Lerp(Vector) "1.000000,1.000000,1.000000" "2.000000,2.000000,0.200000" _newtrack_0))
          (Utilities|FlowControl|Delay 5.0)
          (Actor|DestroyActor))))))

(fn ConstructionScript)