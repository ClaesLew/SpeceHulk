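; BP_Egg is a destructible enemy egg that spawns AI larvae, triggered by player overlap.
; A self-calling delayed loop uses a FlipFlop to alternate between two spawn points while life remains and Sleep is off.
; Leaving the trigger sets Sleep, and entering calls the loop before clearing it.
; Projectile hits drain life; at zero, a timeline squashes the egg mesh and a delay precedes destruction.
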(event OnComponentBeginOverlap(Spawntrigger)
  (params (OverlappedComponent :type Primitive%20Component%20Object%20Reference) (OtherActor :type Actor%20Object%20Reference) (OtherComp :type Primitive%20Component%20Object%20Reference) (OtherBodyIndex :type Integer) (bFromSweep :type Boolean) (SweepResult :type Hit%20Result%20Structure%20%28by%20ref%29))
  (Utilities|Casting|CastToCore_PlayerCharacter OtherActor)
  (CallFunction|SpawnLarvae)
  (Variables|Default|SetbSleep false))

(event OnComponentEndOverlap(Spawntrigger)
  (params (OverlappedComponent :type Primitive%20Component%20Object%20Reference) (OtherActor :type Actor%20Object%20Reference) (OtherComp :type Primitive%20Component%20Object%20Reference) (OtherBodyIndex :type Integer))
  (Utilities|Casting|CastToCore_PlayerCharacter OtherActor)
  (Variables|Default|SetbSleep true))

(event OnComponentHit(Collision)
  (params (HitComponent :type Primitive%20Component%20Object%20Reference) (OtherActor :type Actor%20Object%20Reference) (OtherComp :type Primitive%20Component%20Object%20Reference) (NormalImpulse :type Vector :default "0, 0, 0") (Hit :type Hit%20Result%20Structure%20%28by%20ref%29))
  (bind _life (Variables|Default|GetLife))
  (Utilities|Casting|CastToFirstPersonProjectile OtherActor)
  (Math|Integer|DecrementInt _life
    (:%20%20
      (if (== _life 0)
        (CallFunction|DEATH)))))

(event Custom|SpawnLarvae
  (if (not (Variables|Default|GetbSleep))
    (if (not (<= (Variables|Default|GetLife) 0))
      (Utilities|FlowControl|Delay 3.0)
      (Utilities|FlowControl|FlipFlop
        (:A
          (Game|SpawnActorfromClass "/Game/Root/Core/AI/AI_Larvae_Pawn.AI_Larvae_Pawn_C" (Transformation|GetWorldTransform (Variables|Default|GetSpawn)) "AlwaysSpawn" 0 0))
        (:B
          (Game|SpawnActorfromClass "/Game/Root/Core/AI/AI_Larvae_Pawn.AI_Larvae_Pawn_C" (Transformation|GetWorldTransform (Variables|Default|GetSpawn1)) "AlwaysSpawn" 0 0)))
      (CallFunction|SpawnLarvae))))

(event Custom|DEATH
  (Utilities|FlowControl|Sequence
    (:then_0
      (bind _alpha (Timeline|Timeline_0 Stop)
        (:Update
          (Transformation|SetRelativeScale3D (Variables|Default|GetEggs) (Math|Vector|Lerp(Vector) "1.000000,1.000000,1.000000" "1.000000,1.000000,1.050000" _alpha)))))
    (:then_1
      (bind _newtrack_0 (Timeline|Deathanim Play)
        (:Update
          (Transformation|SetRelativeScale3D (Variables|Default|GetEggs) (Math|Vector|Lerp(Vector) "1.000000,1.000000,1.000000" "2.000000,2.000000,0.200000" _newtrack_0))
          (Utilities|FlowControl|Delay 5.0)
          (Actor|DestroyActor))))))

(fn ConstructionScript)