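; BP_Larvae is a shootable larva enemy that loses health when struck by a FirstPersonProjectile.
; Each projectile hit destroys the projectile and decrements Hitpoints, triggering DEATH once they reach zero.
; DEATH uses a timeline to rotate the skeletal mesh over by lerping its relative rotation, then destroys the actor after a short delay.
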(event Custom|DEATH
  (bind _newtrack_0 (Timeline|Timeline_0 Play)
    (:Update
      (Transformation|SetRelativeRotation (Variables|Default|GetSkeletalMesh) (Math|Rotator|Lerp(Rotator) "0, 0, 0" "180.000000, 0, 0" _newtrack_0) false false))
    (:Finished
      (Utilities|FlowControl|Delay 2.0)
      (Actor|DestroyActor))))

(event Collision|EventHit
  (params (MyComp :type Primitive%20Component%20Object%20Reference) (Other :type Actor%20Object%20Reference) (OtherComp :type Primitive%20Component%20Object%20Reference) (bSelfMoved :type Boolean) (HitLocation :type Vector :default "0, 0, 0") (HitNormal :type Vector :default "0, 0, 0") (NormalImpulse :type Vector :default "0, 0, 0") (Hit :type Hit%20Result%20Structure%20%28by%20ref%29))
  (bind _hitpoints (Variables|Default|GetHitpoints))
  (bind _asfirst_person_projectile (Utilities|Casting|CastToFirstPersonProjectile Other))
  (Actor|DestroyActor _asfirst_person_projectile)
  (Math|Integer|DecrementInt _hitpoints
    (:%20%20
      (if (<= _hitpoints 0)
        (CallFunction|DEATH)))))

(fn ConstructionScript)